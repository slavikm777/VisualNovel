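; StateTree task that shows the dialogue display widget while its state is active.
; On entering, it creates WBP_DialogueDisplay, adds it to the viewport, focuses it with UI-only input and shows the mouse cursor.
; On exit, it removes and clears the widget, then restores game-only input and hides the cursor.
; The task never calls Finish Task itself.
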(event EventLatentEnterState
  (params (Transition :type State%20Tree%20Transition%20Result%20Structure%20%28by%20ref%29))
  (bind _returnvalue (Game|GetPlayerController 0))
  (bind _returnvalue_2 (UserInterface|CreateWidget "/Game/UI/WBP_DialogueDisplay.WBP_DialogueDisplay_C"))
  (bind _output_get (Variables|Output|SetDisplay _returnvalue_2))
  (UserInterface|Viewport|AddtoViewport _output_get 0)
  (Input|SetInputModeUIOnly _returnvalue (Variables|Output|GetDisplay) "DoNotLock" false)
  (Variables|/Script/Engine.PlayerController|SetbShowMouseCursor _returnvalue true))

(event EventExitState
  (params (Transition :type State%20Tree%20Transition%20Result%20Structure%20%28by%20ref%29))
  (bind _returnvalue (Game|GetPlayerController 0))
  (bind _display (Variables|Output|GetDisplay)
    (:then
      (Widget|RemovefromParent _display)
      (Variables|Output|SetDisplay 0))
    (:else
      _))
  (Utilities|IsValid _returnvalue
    (:Is%20Valid
      (Input|SetInputModeGameOnly _returnvalue false)
      (Variables|/Script/Engine.PlayerController|SetbShowMouseCursor _returnvalue false))))